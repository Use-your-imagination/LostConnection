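; Default ranged enemy bot Blueprint that handles reload state and forwards reload and death visual events.
; Reload start and end events toggle IsReloading, with the end event also calling RunReloadLogic.
; Visual events pass the enemy itself to ReloadVisual and DeathInit, while death timeline updates feed their value into DeathUpdate as a parameter.
; The graph only wires events, with the visual logic defined outside it and an empty construction script.
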(event Custom|ReloadEnd
  (Variables|Default|SetisReloading false)
  (Class|BaseCharacter|RunReloadLogic))

(event Custom|ReloadStart
  (Variables|Default|SetisReloading true))

(event EventReloadEventVisual
  (CallFunction|ReloadVisual self))

(event EventDeathTimelineUpdate
  (params (value :type Float%20%28single-precision%29))
  (CallFunction|DeathUpdate self value))

(event EventDeathEventVisual
  (CallFunction|DeathInit self))

(fn ConstructionScript)