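; BP_DefaultEnemy is an AI-controlled enemy bot that handles reload state plus reload and death visuals.
; On BeginPlay it runs the parent logic and writes itself to the Blackboard as SelfActor, if one exists.
; Reload events toggle IsReloading and run the reload logic on completion.
; Visual events pass the bot to ReloadVisual and DeathInit, while death timeline updates feed their value to DeathUpdate.
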(event Custom|ReloadEnd
  (Variables|Default|SetisReloading false)
  (Class|BaseCharacter|RunReloadLogic))

(event Custom|ReloadStart
  (Variables|Default|SetisReloading true))

(event EventReloadEventVisual
  (CallFunction|ReloadVisual self))

(event EventBeginPlay
  (bind _self self)
  (bind _returnvalue (AI|GetBlackboard _self))
  (|CallParentFunction)
  (Utilities|IsValid _returnvalue
    (:Is%20Valid
      (AI|Components|Blackboard|SetValueasObject _returnvalue (Utilities|Name|MakeLiteralName "SelfActor") _self))))

(event EventDeathTimelineUpdate
  (params (value :type Float%20%28single-precision%29))
  (CallFunction|DeathUpdate self value))

(event EventDeathEventVisual
  (CallFunction|DeathInit self))

(fn ConstructionScript)