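; BP_DefaultEnemyAI is the default AI controller for enemies, running DefaultEnemyBehaviourTree on BeginPlay.
; Its AIPerception update handler ignores actors that are not BaseCharacters.
; A successfully sensed ally-flagged character is written to the DetectedPlayer blackboard key.
; Any other BaseCharacter update, whether a lost stimulus or a non-ally, clears that key.
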(event OnTargetPerceptionUpdated(AIPerception)
  (params (Actor :type Actor%20Object%20Reference) (Stimulus :type AI%20Stimulus%20Structure))
  (bind _returnvalue (Utilities|Name|MakeLiteralName "DetectedPlayer"))
  (bind _blackboard (Variables|Default|GetBlackboard))
  (bind _asbase_character (Utilities|Casting|CastToBaseCharacter Actor))
  (if (and (Class|LostConnectionCharacter|GetIsAlly _asbase_character) (.bSuccessfullySensed (Utilities|Struct|BreakAIStimulus Stimulus)))
    (AI|Components|Blackboard|SetValueasObject _blackboard _returnvalue _asbase_character)
    (else
      (AI|Components|Blackboard|SetValueasObject _blackboard _returnvalue 0))))

(event EventBeginPlay
  (AI|RunBehaviorTree "/Game/AI/Enemies/BehaviourTrees/Default/DefaultEnemyBehaviourTree.DefaultEnemyBehaviourTree"))

(fn ConstructionScript)