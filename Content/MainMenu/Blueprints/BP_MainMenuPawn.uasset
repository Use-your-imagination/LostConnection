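; Main menu pawn with a debug-style key trigger that animates the materials of the menu's buttons.
; Pressing Z plays the Butterat timeline, which each update loops over the current BP_MainMenu's items and writes its value to the "Test" scalar on each button's normal-style dynamic material.
; A Settings timeline for moving the camera along a spline is present but never runs.
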(event Input|KeyboardEvents|Z
  (params (Key :type Key%20Structure :default "None"))
  (:Pressed
    (bind _butterattime (Timeline|Butterat PlayFromStart)
      (:Update
        (bind _asbp_main_menu (Utilities|Casting|CastToBP_MainMenu (Variables|/Game/MainMenu/UI/BP_MainMenuUI.BP_MainMenuUI_C|GetCurrentMenu (Variables|Default|GetUI))))
        (for _index (range 0 (Class|ListView|GetNumItems (Variables|/Game/UI/Menu/BP_BaseMenu.BP_BaseMenu_C|GetMenu _asbp_main_menu)))
          (bind _asmaterial_instance_dynamic (Utilities|Casting|CastToMaterialInstanceDynamic (.ResourceObject (Utilities|Struct|BreakSlateBrush (.Normal (Utilities|Struct|BreakButtonStyle (Variables|/Script/UMG.Button|GetWidgetStyle (Variables|/Game/UI/Menu/MenuItems/BP_BaseMenuItem.BP_BaseMenuItem_C|GetItemButton (Default|GetItem _asbp_main_menu _index)))))))))
          (Rendering|Material|SetScalarParameterValue _asmaterial_instance_dynamic "Test" _butterattime :!class /Script/Engine.MaterialInstanceDynamic))))))

(fn ConstructionScript)