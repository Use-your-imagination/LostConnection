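; Loot function for Legendary weapons that turns loot points into a value for that rarity tier.
; It reports the Legendary rarity and its name alongside the main curve.
; The curve stays at zero up to a threshold set by GlobalScale, then rises quadratically with no upper clamp, so Legendary only registers at high loot points.
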(fn GetLootName
  (return "LegendaryRarityName"))

(fn GetWeaponRarity
  (return "legendary"))

(fn MainFunction
  (params (LootPoints :type Integer))
  (bind _globalscale (Variables|Default|GetGlobalScale))
  (return (select (> LootPoints (* (Variables|Default|GetGlobalScale) 4)) (Math|Float|Power (/ (Math|Conversions|ToFloat(Integer) (- (* _globalscale 4) LootPoints)) (Math|Conversions|ToFloat(Integer) (* _globalscale 12))) 2.0) 0.0)))