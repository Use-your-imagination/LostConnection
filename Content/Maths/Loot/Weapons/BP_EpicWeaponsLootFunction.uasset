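; BP_EpicWeaponsLootFunction is the loot function for Epic rarity weapons, supplying the tier's name, rarity and a value curve over loot points.
; MainFunction returns zero until loot points exceed GlobalScale, then follows a squared curve of the scaled excess.
; It constructs the Legendary weapons function and caps that curve at one minus the Legendary result, so Epic only takes what Legendary leaves.
; GetRange returns zero for both soft and hard limits.
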(fn GetLootName
  (return "EpicRarityName"))

(fn GetWeaponRarity
  (return "epic"))

(fn MainFunction
  (params (LootPoints :type Integer))
  (bind _globalscale (Variables|Default|GetGlobalScale))
  (bind _returnvalue (- _globalscale LootPoints))
  (bind _returnvalue_2 (* _globalscale 8))
  (bind _returnvalue_3 (Math|Conversions|ToFloat(Integer) _returnvalue_2))
  (bind _returnvalue_4 (Math|Conversions|ToFloat(Integer) _returnvalue))
  (bind _returnvalue_5 (/ _returnvalue_4 _returnvalue_3))
  (bind _returnvalue_6 (Math|Float|Power _returnvalue_5 2.0))
  (bind _returnvalue_7 (Game|ConstructObjectfromClass "/Game/Maths/Loot/Weapons/BP_LegendaryWeaponsLootFunction.BP_LegendaryWeaponsLootFunction_C" self))
  (return (select (> LootPoints (Variables|Default|GetGlobalScale)) (select (< (- 1.0 (CallFunction|MainFunction _returnvalue_7 LootPoints)) _returnvalue_6) (- 1.0 (CallFunction|MainFunction _returnvalue_7 LootPoints)) _returnvalue_6) 0.0)))

(fn GetRange
  (return 0 0))