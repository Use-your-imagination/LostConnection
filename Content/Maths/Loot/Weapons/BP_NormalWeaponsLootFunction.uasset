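; BP_NormalWeaponsLootFunction is the Normal-rarity weapon loot function, mapping loot points to that rarity's share, with a name, rarity and zero range.
; MainFunction constructs the Rare and Epic loot function objects and subtracts their combined results from one.
; It returns the lesser of that remainder and a quadratic curve of loot points over GlobalScale, so Normal depends on what the higher tiers leave.
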(fn GetLootName
  (return "NormalRarityName"))

(fn GetWeaponRarity
  (return "normal"))

(fn GetRange
  (return 0 0))

(fn MainFunction
  (params (LootPoints :type Integer))
  (bind _returnvalue (Math|Conversions|ToFloat(Integer) LootPoints))
  (bind _self self)
  (bind _globalscale (Variables|Default|GetGlobalScale))
  (bind _returnvalue_2 (Math|Conversions|ToFloat(Integer) _globalscale))
  (bind _returnvalue_3 (/ _returnvalue _returnvalue_2))
  (bind _returnvalue_4 (Math|Float|Power _returnvalue_3 2.0))
  (bind _returnvalue_5 (Game|ConstructObjectfromClass "/Game/Maths/Loot/Weapons/BP_RareWeaponsLootFunction.BP_RareWeaponsLootFunction_C" _self))
  (bind _returnvalue_6 (Game|ConstructObjectfromClass "/Game/Maths/Loot/Weapons/BP_EpicWeaponsLootFunction.BP_EpicWeaponsLootFunction_C" _self))
  (return (select (< (- 1.0 (+ (CallFunction|MainFunction _returnvalue_6 LootPoints) (CallFunction|MainFunction _returnvalue_5 LootPoints))) _returnvalue_4) (- 1.0 (+ (CallFunction|MainFunction _returnvalue_6 LootPoints) (CallFunction|MainFunction _returnvalue_5 LootPoints))) _returnvalue_4)))