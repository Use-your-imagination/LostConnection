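; Loot function for the Rare weapon tier, giving its name, rarity and drop chance for a given number of loot points.
; The chance is zero up to GlobalScale, then rises quadratically with the points beyond it.
; It constructs the Epic and Legendary loot functions and caps the Rare chance at whatever share those two leave out of 1.
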(fn GetLootName
  (return "RareRarityName"))

(fn GetWeaponRarity
  (return "rare"))

(fn MainFunction
  (params (LootPoints :type Integer))
  (bind _self self)
  (bind _globalscale (Variables|Default|GetGlobalScale))
  (bind _returnvalue (* _globalscale 1))
  (bind _returnvalue_2 (* _globalscale 3))
  (bind _returnvalue_3 (Math|Conversions|ToFloat(Integer) _returnvalue_2))
  (bind _returnvalue_4 (- _returnvalue LootPoints))
  (bind _returnvalue_5 (Math|Conversions|ToFloat(Integer) _returnvalue_4))
  (bind _returnvalue_6 (/ _returnvalue_5 _returnvalue_3))
  (bind _returnvalue_7 (Math|Float|Power _returnvalue_6 2.0))
  (bind _returnvalue_8 (Game|ConstructObjectfromClass "/Game/Maths/Loot/Weapons/BP_EpicWeaponsLootFunction.BP_EpicWeaponsLootFunction_C" _self))
  (bind _returnvalue_9 (Game|ConstructObjectfromClass "/Game/Maths/Loot/Weapons/BP_LegendaryWeaponsLootFunction.BP_LegendaryWeaponsLootFunction_C" _self))
  (return (select (> LootPoints (Variables|Default|GetGlobalScale)) (select (< (- 1.0 (+ (CallFunction|MainFunction _returnvalue_8 LootPoints) (CallFunction|MainFunction _returnvalue_9 LootPoints))) _returnvalue_7) (- 1.0 (+ (CallFunction|MainFunction _returnvalue_8 LootPoints) (CallFunction|MainFunction _returnvalue_9 LootPoints))) _returnvalue_7) 0.0)))