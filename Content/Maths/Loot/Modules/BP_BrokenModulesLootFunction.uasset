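; BP_BrokenModulesLootFunction defines the loot curve for Broken-quality modules.
; It supplies the quality's name key and Broken enum value, along with a breakpoint starting at zero with a unit multiplier.
; Its unrefined main function is an inverted parabola of loot points normalized by GlobalScale, so the value falls from one as points rise, reaching zero at GlobalScale.
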(fn GetLootName
  (return "BrokenQualityName"))

(fn GetModuleQuality
  (return "broken"))

(fn MainFunctionUnref
  (params (LootPoints :type Integer))
  (return (- 1.0 (Math|Float|Power (/ LootPoints (Variables|Default|GetGlobalScale)) 2.0))))

(fn FuncBreakPoint
  (return 0 1))