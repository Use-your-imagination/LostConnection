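; Base weapon-module loot function that converts loot points into a drop chance, also available as a percentage.
; Past a scaled breakpoint from FuncBreakPoint, chance grows quadratically; otherwise it is zero.
; Suber constructs each class preceding this one in LootMassive and sums their chances recursively through MainFunction.
; The result is capped at the probability those earlier entries leave unused and clamped to non-negative, so array order sets priority.
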(fn FuncBreakPoint
  (return 0 1))

(fn MainFunctionUnref
  (params (LootPoints :type Integer))
  (bind (_startbreakpoint _funcmulti) (CallFunction|FuncBreakPoint))
  (bind _globalscale (Variables|Default|GetGlobalScale))
  (return (Math|Float|Power (/ (- (* _globalscale _startbreakpoint) LootPoints) (* _globalscale _funcmulti)) 2.0)))

(fn Suber
  (params (LootPoints :type Integer))
  (for _array_element (Variables|Default|GetLootMassive)
    (if (== _array_element (Utilities|GetClass self))
      (return (LocalVariables|GetChance))
      (else
        (bind _returnvalue (Game|ConstructObjectfromClass _array_element))
        (LocalVariables|SetChance (+ (CallFunction|MainFunction _returnvalue LootPoints) (LocalVariables|GetChance)))))))

(fn MainFunction
  (params (LootPoints :type Integer))
  (bind _chance (CallFunction|MainFunctionUnref LootPoints))
  (bind _returnchance (CallFunction|Suber LootPoints))
  (return (Math|Float|Max(Float) (Math|Float|SelectFloat (Math|Float|SelectFloat (- 1.0 _returnchance) _chance (< (- 1.0 _returnchance) _chance)) 0.0 (> LootPoints (* (Variables|Default|GetGlobalScale) (.StartBreakpoint (CallFunction|FuncBreakPoint))))) 0.0)))

(fn CalculateLootChance
  (params (lootPoints :type Integer))
  (return (* (CallFunction|MainFunction lootPoints) 1e+02)))