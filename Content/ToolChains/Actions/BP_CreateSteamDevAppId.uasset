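; A toolchain action that creates the steam_appid.txt file for a staged Windows build of the project.
; Initialization parses the .env file in the project directory as JSON and reads its appId field.
; Execute writes that ID as text into the staged build's Binaries/Win64 folder.
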(event EventExecute
  (Class|AutomationToolchainLibrary|CreateFile (Class|AutomationToolchainLibrary|AppendPath (Class|AutomationToolchainLibrary|GetPathtoStagedBuildsFolder) "Windows" (Class|AutomationToolchainLibrary|GetProjectName) "Binaries" "Win64") "steam_appid" "txt" (Utilities|String|ToString(Integer) (Variables|Default|GetAppId))))

(event EventInitialization
  (Variables|Default|SetAppId (Class|JsonLibrary|GetJsonInteger "appId" (.ReturnValue (Class|JsonLibrary|ParseJsonFile (Utilities|String|Append (Class|KismetSystemLibrary|GetProjectDirectory) ".env"))))))