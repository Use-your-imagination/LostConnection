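; Tool-chain distribution action that publishes the LostConnection Windows build as a GitHub release.
; Initialization reads the GitHub token from the project's .env file.
; Execute shells out to curl to create a release tagged with the project version and linking its patch notes, saving the response to response.json.
; It then uploads LostConnection.zip to the returned upload_url and deletes the response file.
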(event EventExecute
  (Class|AutomationToolchainLibrary|ExecuteShellCommand "curl" (CallFunction|GenerateParameters) (CallFunction|GetPathtoBuildFolder))
  (CallFunction|UploadZip)
  (CallFunction|Clean))

(event EventInitialization
  (Variables|Default|SetToken (Class|JsonLibrary|GetJsonString "token" (.ReturnValue (Class|JsonLibrary|ParseJsonFile (Utilities|String|Append (Class|KismetSystemLibrary|GetProjectDirectory) ".env"))))))

(fn GenerateParameters
  (bind _returnvalue (Class|AutomationToolchainLibrary|GetProjectVersion))
  (return (Utilities|String|Append "-X POST " "-H \"Accept: application/vnd.github.v3+json\" " (Utilities|String|ToString(Text) (Utilities|Text|FormatText "-H \"Authorization: token {Token}\" " (Variables|Default|GetToken))) "https://api.github.com/repos/Use-your-imagination/LostConnection/releases?name=LostConnection.zip " (Utilities|String|Append "-d \"{" (Utilities|String|ToString(Text) (Utilities|Text|FormatText "\\\"tag_name\\\":\\\"{VersionName}\\\",\\\"target_commitish\\\":\\\"master\\\",\\\"name\\\":\\\"{VersionName}\\\",\\\"body\\\":\\\"[Patch notes](https://use-your-imagination.github.io/LostConnection/LostConnection_{Version}.html)\\\",\\\"draft\\\":false,\\\"prerelease\\\":false,\\\"generate_release_notes\\\":false" _returnvalue (Utilities|String|Replace _returnvalue "v"))) "}\" ") "-o response.json")))

(fn UploadZip
  (bind _data (Class|AutomationToolchainLibrary|ReadFile (Class|AutomationToolchainLibrary|AppendPath (CallFunction|GetPathtoBuildFolder) "response.json")))
  (if (.result (Class|JsonLibrary|TryGetJsonString "upload_url" (.ReturnValue (Class|JsonLibrary|ParseJson _data))))
    (Class|AutomationToolchainLibrary|ExecuteShellCommand "curl" (Utilities|String|Append "-X POST " "-H \"Accept: application/vnd.github.v3+json\" " (Utilities|String|ToString(Text) (Utilities|Text|FormatText "-H \"Authorization: token {Token}\" " (Variables|Default|GetToken))) (Utilities|String|Replace (.ReturnValue (Class|JsonLibrary|TryGetJsonString "upload_url" (.ReturnValue (Class|JsonLibrary|ParseJson _data)))) "{?name,label}" "?name=LostConnection.zip ") "-H \"Content-Type: application/zip\" " "--data-binary @LostConnection.zip ") (CallFunction|GetPathtoBuildFolder))))

(fn GetPathtoBuildFolder
  (return (Class|AutomationToolchainLibrary|AppendPath (Class|AutomationToolchainLibrary|GetPathtoStagedBuildsFolder) "Windows")))

(fn Clean
  (Class|AutomationToolchainLibrary|DeleteFile (Class|AutomationToolchainLibrary|AppendPath (CallFunction|GetPathtoBuildFolder) "response.json")))