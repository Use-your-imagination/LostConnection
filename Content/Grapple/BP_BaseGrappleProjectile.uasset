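; Base grapple projectile that limits how far it can travel and reports to its Handler when it goes too far.
; On authority only, it stores its start location at BeginPlay and checks the distance from that point every Tick.
; Once that distance exceeds MaxDistance, LimitReached notifies the Handler and destroys the projectile.
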(event Custom|LimitReached
  (Default|OnLimitReached (Variables|Default|GetHandler))
  (Actor|DestroyActor))

(event EventTick
  (params (DeltaSeconds :type Float%20%28single-precision%29))
  (Networking|SwitchHasAuthority
    (:Authority
      (if (> (Math|Vector|VectorLength (- (Variables|Default|GetStartLocation) (Transformation|GetActorLocation))) (Variables|Default|GetMaxDistance))
        (CallFunction|LimitReached)))))

(event EventBeginPlay
  (Networking|SwitchHasAuthority
    (:Authority
      (Variables|Default|SetStartLocation (Transformation|GetActorLocation)))))

(fn ConstructionScript)