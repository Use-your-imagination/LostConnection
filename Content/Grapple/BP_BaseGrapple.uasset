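; Server-authoritative grapple actor that swings a BaseDrone from an anchor point on a physics-driven rope.
; At BeginPlay it builds a Hinge, Anchor, Hand constraint and simulated Capsule chain, then attaches the drone to the capsule.
; Tick wraps the rope around obstacles using two-way sphere traces, adding pivots and shortening the limit, and optionally takes up slack.
; Below minimum length it self-destructs; EndPlay applies the last velocity to the drone as force.
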(event EventBeginPlay
  (Networking|SwitchHasAuthority
    (:Authority
      (CallFunction|RealiseTarget)
      (CallFunction|ComponentSetup)
      (CallFunction|VariablesSetup))))

(event EventTick
  (params (DeltaSeconds :type Float%20%28single-precision%29))
  (bind _output (CallFunction|GetLastAnchor))
  (bind _output_2 (CallFunction|GetLastAnchor))
  (bind _hand (Variables|Default|GetHand))
  (bind _capsule (Variables|Default|GetCapsule))
  (bind _hand_2 (Variables|Default|GetHand))
  (bind _returnvalue (Transformation|GetWorldLocation _capsule))
  (bind _returnvalue_2 (- _returnvalue _output))
  (bind _returnvalue_3 (Math|Vector|VectorLength _returnvalue_2))
  (Networking|SwitchHasAuthority
    (:Authority
      (bind _returnvalue_4 (Class|PhysicsConstraintComponent|GetConstraint (Variables|Default|GetHand)))
      (bind _limit (Class|ConstraintInstanceBlueprintLibrary|GetLinearLimits _returnvalue_4))
      (if (> _limit (Variables|Default|GetGrappleMinHand))
        (Utilities|FlowControl|Sequence
          (:then_0
            (bind (_overlappoint _and) (CallFunction|FeedbackTrace))
            (if _and
              (bind _returnvalue_5 (Class|PhysicsConstraintComponent|GetConstraint _hand))
              (bind _limit_2 (Class|ConstraintInstanceBlueprintLibrary|GetLinearLimits _returnvalue_5))
              (Class|PhysicsConstraintComponent|SetConstraintReferencePosition _hand "Frame1" (- (Transformation|GetActorLocation) _output_2))
              (Class|PhysicsConstraintComponent|SetLinearXLimit _hand "LCM_Limited" (- _limit_2 (Math|Vector|VectorLength (- _overlappoint _output_2))))
              (Utilities|Array|Add (Variables|Default|GetAnchorArray) _overlappoint)))
          (:then_1
            (Variables|Default|SetLastSpeed (Transformation|GetComponentVelocity (Variables|Default|GetCapsule)))
            (if (Variables|Default|GetUpdateLength)
              (bind _returnvalue_6 (Class|PhysicsConstraintComponent|GetConstraint _hand_2))
              (bind _limit_3 (Class|ConstraintInstanceBlueprintLibrary|GetLinearLimits _returnvalue_6))
              (Class|PhysicsConstraintComponent|SetLinearXLimit _hand_2 "LCM_Limited" (Math|Float|SelectFloat _returnvalue_3 _limit_3 (< _returnvalue_3 _limit_3))))))
        (else
          (Actor|DestroyActor))))))

(event EventEndPlay
  (params (EndPlayReason :type EEndPlayReason%20Enum :default "Destroyed"))
  (bind _lastspeed (Variables|Default|GetLastSpeed))
  (bind _drone (Variables|Default|GetDrone))
  (bind _charactermovement (Variables|/Script/Engine.Character|GetCharacterMovement _drone))
  (bind _capsulecomponent (Variables|/Script/Engine.Character|GetCapsuleComponent _drone))
  (Networking|SwitchHasAuthority
    (:Authority
      (Physics|SetSimulatePhysics _capsulecomponent false)
      (Transformation|DetachFromActor "KeepWorld" "KeepWorld" "KeepWorld")
      (Transformation|SetWorldRotation _capsulecomponent (Math|Rotator|MakeRotator 0.0 0.0 (.yaw (Math|Conversions|RotationFromXVector _lastspeed))) false false)
      (Components|Movement|StopMovementImmediately _charactermovement)
      (Physics|AddForce _charactermovement (* _lastspeed (Variables|Default|GetResetSpeendMultiplier))))))

(fn ConstructionScript)

(fn ComponentSetup
  (Utilities|FlowControl|Sequence
    (:then_0
      (bind _returnvalue (Game|AddComponentbyClass "/Script/Engine.PhysicsConstraintComponent" false))
      (bind _output_get (Variables|Default|SetHinge _returnvalue))
      (bind _returnvalue_2 (Game|AddComponentbyClass "/Script/Engine.SphereComponent" false))
      (bind _output_get_2 (Variables|Default|SetAnchor _returnvalue_2))
      (bind _returnvalue_3 (Game|AddComponentbyClass "/Script/Engine.PhysicsConstraintComponent" false))
      (bind _output_get_3 (Variables|Default|SetHand _returnvalue_3))
      (bind _returnvalue_4 (Game|AddComponentbyClass "/Script/Engine.CapsuleComponent" false))
      (bind _output_get_4 (Variables|Default|SetCapsule _returnvalue_4)))
    (:then_1
      (Transformation|AttachComponentToComponent _output_get_2 _output_get "None" "KeepRelative" "KeepRelative" "KeepRelative" true)
      (Transformation|AttachComponentToComponent _output_get_3 _output_get_2 "None" "KeepRelative" "KeepRelative" "KeepRelative" true)
      (Transformation|AttachComponentToComponent _output_get_4 _output_get_3 "None" "KeepRelative" "KeepRelative" "KeepRelative" true))
    (:then_2
      (CallFunction|HingeSetup)
      (CallFunction|AnchorSetup)
      (CallFunction|CapsuleSetup)
      (CallFunction|HandSetup))))

(fn RealiseTarget
  (bind _asbase_drone (Utilities|Casting|CastToBaseDrone (Variables|Default|GetInstigator)))
  (Variables|Default|SetDrone _asbase_drone)
  (bind _asbp_base_grapple_handler (Utilities|Casting|CastToBP_BaseGrappleHandler (Variables|Default|Gethandler)))
  (Variables|Default|SetCastedHandler _asbp_base_grapple_handler))

(fn HingeSetup
  (bind _hinge (Variables|Default|GetHinge))
  (Class|PhysicsConstraintComponent|SetConstrainedComponents _hinge 0 "None" (Variables|Default|GetAnchor) "None")
  (Class|PhysicsConstraintComponent|SetAngularTwistLimit _hinge "ACM_Locked" 0.0)
  (Class|ActorComponent|SetIsReplicated _hinge true)
  (bind _returnvalue (Class|PhysicsConstraintComponent|GetConstraint _hinge))
  (Class|ConstraintInstanceBlueprintLibrary|SetLinearLimits _returnvalue "LCM_Locked" "LCM_Locked" "LCM_Locked" 0.0))

(fn AnchorSetup
  (bind _anchor (Variables|Default|GetAnchor))
  (Rendering|SetVisibility _anchor false false)
  (Physics|SetSimulatePhysics _anchor true)
  (Collision|SetCollisionResponsetoAllChannels _anchor "ECR_Ignore")
  (Class|ActorComponent|SetIsReplicated _anchor true))

(fn HandSetup
  (bind _hand (Variables|Default|GetHand))
  (Class|PhysicsConstraintComponent|SetConstrainedComponents _hand (Variables|Default|GetAnchor) "None" (Variables|Default|GetCapsule) "None")
  (Class|PhysicsConstraintComponent|SetAngularSwing1Limit _hand "ACM_Locked" 0.0)
  (Class|PhysicsConstraintComponent|SetAngularSwing2Limit _hand "ACM_Locked" 0.0)
  (Class|PhysicsConstraintComponent|SetAngularTwistLimit _hand "ACM_Locked" 0.0)
  (Class|PhysicsConstraintComponent|SetLinearXLimit _hand "LCM_Limited" (Math|Vector|VectorLength (- (Transformation|GetActorLocation (Variables|Default|GetDrone)) (Transformation|GetActorLocation))))
  (Class|PhysicsConstraintComponent|SetConstraintReferencePosition _hand "Frame1" (Math|Vector|MakeVector 0.0 0.0 0.0))
  (bind _returnvalue (Class|PhysicsConstraintComponent|GetConstraint _hand))
  (Class|ConstraintInstanceBlueprintLibrary|SetLinearSoftLimitParams _returnvalue true 1e+03 0.0 0.0 0.0)
  (Class|ConstraintInstanceBlueprintLibrary|SetLinearPositionDrive _returnvalue true false false)
  (Class|ConstraintInstanceBlueprintLibrary|SetLinearDriveParams _returnvalue 1e+01 0.0 0.0)
  (Class|ActorComponent|SetIsReplicated _hand true))

(fn CapsuleSetup
  (bind _capsule (Variables|Default|GetCapsule))
  (bind _drone (Variables|Default|GetDrone))
  (bind _capsulecomponent (Variables|/Script/Engine.Character|GetCapsuleComponent _drone))
  (Components|Capsule|SetCapsuleHalfHeight _capsule (Components|Capsule|GetScaledCapsuleHalfHeight _capsulecomponent) true)
  (Components|Capsule|SetCapsuleRadius _capsule (Components|Capsule|GetScaledCapsuleRadius _capsulecomponent) true)
  (Physics|SetSimulatePhysics _capsule true)
  (Collision|SetCollisionEnabled _capsule "PhysicsOnly")
  (Collision|SetCollisionResponsetoAllChannels _capsule "ECR_Ignore")
  (Development|SetHiddeninGame _capsule true false)
  (Physics|AddForce _capsule (* (Transformation|GetVelocity (Variables|Default|GetDrone)) (LocalVariables|GetForceMultiplier)) "None" true)
  (Transformation|SetRelativeLocation _capsule (Transformation|GetActorLocation (Variables|Default|GetDrone)) false true)
  (Transformation|AttachComponentToComponent (Variables|Default|GetDrone) _capsule "None" "KeepWorld" "KeepWorld" "KeepWorld" true)
  (Class|ActorComponent|SetIsReplicated _capsule true)
  (Class|PrimitiveComponent|SetMassOverrideinKg _capsule "None" 1e+02 true))

(fn FeedbackTrace
  (bind _output (CallFunction|GetLastAnchor))
  (bind _drone (Variables|Default|GetDrone))
  (bind _precisionradius (Variables|Default|GetPrecisionRadius))
  (bind _draw_debug_type (Variables|Default|GetDraw%20Debug%20Type))
  (bind _returnvalue (Transformation|GetActorLocation _drone))
  (bind _array (Utilities|Array|MakeArray _drone))
  (bind (_outhit _returnvalue_2) (Collision|SphereTraceByChannel _returnvalue _output _precisionradius "TraceTypeQuery1" false _array _draw_debug_type true "(R=0.965394,G=0.000000,B=1.000000,A=1.000000)" "(R=1.000000,G=0.904667,B=0.000000,A=1.000000)"))
  (bind (_outhit_2 _returnvalue_3) (Collision|SphereTraceByChannel _output _returnvalue _precisionradius "TraceTypeQuery1" false _array _draw_debug_type))
  (return (+ (/ (+ (.location _outhit) (.location _outhit_2)) 2) (* (/ (+ (.normal _outhit_2) (.normal _outhit)) (Math|Vector|VectorLength (+ (.normal _outhit_2) (.normal _outhit)))) (Variables|Default|GetPrecisionRadius))) (and _returnvalue_3 _returnvalue_2)))

(fn GetLastAnchor
  (bind _anchorarray (Variables|Default|GetAnchorArray))
  (return (Utilities|Array|Get(acopy) _anchorarray (- (Utilities|Array|Length _anchorarray) 1))))

(fn VariablesSetup
  (Utilities|Array|Add (Variables|Default|GetAnchorArray) (Transformation|GetActorLocation))
  (Variables|Default|SetPrecisionRadius (Variables|/Game/Grapple/BP_BaseGrappleHandler.BP_BaseGrappleHandler_C|GetGrapplePrecisionRad (Variables|Default|GetCastedHandler))))