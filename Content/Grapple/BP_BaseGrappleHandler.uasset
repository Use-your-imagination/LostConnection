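; Base handler for the drone's grapple, turning a button press into a fired projectile and then an anchored grapple actor.
; Press launches a projectile from the follow camera if usable and no grapple exists; otherwise it destroys any existing grapple.
; On hit, SetupGrapple spawns GrappleClass offset along the surface normal, facing the drone.
; Release, limit-reached and break hooks are empty, and the drive-reset and cooldown nodes are disconnected.
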(event Custom|Hit
  (params (SelfActor :type Actor%20Object%20Reference) (OtherActor :type Actor%20Object%20Reference) (NormalImpulse :type Vector) (Hit :type Hit%20Result%20Structure%20%28by%20ref%29))
  (CallFunction|SetupGrapple Hit))

(event Custom|OnLimitReached)

(event EventGrappleActionPress
  (if (and (Class|Cooldownable|IsUsable) (not (Utilities|IsValid (Variables|Default|GetOwnedGrapple))))
    (bind _returnvalue (Game|SpawnActorfromClass "/Game/Grapple/BP_BaseGrappleProjectile.BP_BaseGrappleProjectile_C" (Transformation|GetWorldTransform (Variables|/Script/LostConnection.BaseDrone|GetFollowCamera (Variables|Default|Getdrone))) "Undefined" 0 self 0))
    (Collision|BindEventtoOnActorHit _returnvalue (delegate Custom|Hit))
    (elif (Utilities|IsValid (Variables|Default|GetOwnedGrapple))
      (Actor|DestroyActor (Variables|Default|GetOwnedGrapple))
      (Variables|Default|SetOwnedGrapple 0))))

(event EventGrappleActionRelease
  (if (Utilities|IsValid (Variables|Default|GetOwnedGrapple))
    _))

(fn SetupGrapple
  (params (HitResult :type Hit%20Result%20Structure))
  (bind (_bblockinghit _binitialoverlap _time _distance _location _impactpoint _normal) (Collision|BreakHitResult HitResult))
  (bind _drone (Variables|Default|Getdrone))
  (bind _grappleprecisionrad (Variables|Default|GetGrapplePrecisionRad))
  (bind _returnvalue (* _normal _grappleprecisionrad))
  (bind _returnvalue_2 (+ _location _returnvalue))
  (bind _returnvalue_3 (Game|SpawnActorfromClass (Variables|Default|GetgrappleClass) (Math|Transform|MakeTransform _returnvalue_2 (Math|Conversions|RotationFromXVector (- (Transformation|GetActorLocation _drone) _returnvalue_2)) "1.000000,1.000000,1.000000") "Undefined" 0 self _drone))
  (Variables|Default|SetOwnedGrapple _returnvalue_3))

(fn InitGrappleBreak)