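; Grapple actor that swings its instigating BaseDrone on a physics component held by a length-limited constraint.
; On authority, Tick runs two-way sphere traces to the latest anchor, adding wrap points at obstructions, moving the constraint reference and shortening the rope.
; UpdateLength lets the limit shrink as the drone closes in; a too-short rope destroys the actor.
; EndPlay detaches and applies the last velocity as a force on the drone's movement.
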(event EventEndPlay
  (params (EndPlayReason :type EEndPlayReason%20Enum :default "Destroyed"))
  (bind _lastspeed (Variables|Default|GetLastSpeed))
  (bind _grappler (Variables|Default|GetGrappler))
  (bind _capsulecomponent (Variables|/Script/Engine.Character|GetCapsuleComponent _grappler))
  (bind _charactermovement (Variables|/Script/Engine.Character|GetCharacterMovement _grappler))
  (Physics|SetSimulatePhysics _capsulecomponent false)
  (Transformation|DetachFromActor "KeepWorld" "KeepWorld" "KeepWorld")
  (Transformation|SetWorldRotation _capsulecomponent (Math|Rotator|MakeRotator 0.0 0.0 (.yaw (Math|Conversions|RotationFromXVector _lastspeed))) false false)
  (Components|Movement|StopMovementImmediately _charactermovement)
  (Physics|AddForce _charactermovement (* _lastspeed 10000)))

(event EventTick
  (params (DeltaSeconds :type Float%20%28single-precision%29))
  (bind _returnvalue (Transformation|GetActorLocation))
  (bind _returnvalue_2 (Transformation|GetActorLocation))
  (bind _anchorarray (Variables|Default|GetAnchorArray))
  (bind _fuckepics (Variables|Default|GetFuckEpics))
  (bind _addedlayer (Variables|Default|GetAddedLayer))
  (bind _grappler (Variables|Default|GetGrappler))
  (bind _returnvalue_3 (Utilities|Array|IsNotEmpty _anchorarray))
  (bind _returnvalue_4 (Utilities|Array|Length _anchorarray))
  (bind _returnvalue_5 (Transformation|GetWorldLocation _fuckepics))
  (bind _returnvalue_6 (- _returnvalue_4 1))
  (bind _returnvalue_7 (- _returnvalue_5 _returnvalue_2))
  (bind _returnvalue_8 (Math|Vector|VectorLength _returnvalue_7))
  (bind _output (Utilities|Array|Get(acopy) _anchorarray _returnvalue_6))
  (bind _returnvalue_9 (select _returnvalue_3 _output _returnvalue))
  (Networking|SwitchHasAuthority
    (:Authority
      (bind _returnvalue_10 (Class|PhysicsConstraintComponent|GetConstraint (Variables|Default|GetAddedLayer)))
      (bind _limit (Class|ConstraintInstanceBlueprintLibrary|GetLinearLimits _returnvalue_10))
      (if (> _limit 9e+01)
        (Utilities|FlowControl|Sequence
          (:then_0
            (bind (_outhit_impactpoint _returnvalue_11) (CallFunction|Trace (Transformation|GetActorLocation _grappler) _returnvalue_9 (Utilities|Array|MakeArray _grappler)))
            (if _returnvalue_11
              (bind _returnvalue_12 (Class|PhysicsConstraintComponent|GetConstraint _addedlayer))
              (bind _limit_2 (Class|ConstraintInstanceBlueprintLibrary|GetLinearLimits _returnvalue_12))
              (Class|PhysicsConstraintComponent|SetConstraintReferencePosition _addedlayer "Frame1" (- (Transformation|GetActorLocation) _returnvalue_9))
              (Class|PhysicsConstraintComponent|SetLinearXLimit _addedlayer "LCM_Limited" (- _limit_2 (Math|Vector|VectorLength (- _outhit_impactpoint _returnvalue_9))))
              (bind _returnvalue_13 (Class|PhysicsConstraintComponent|GetConstraint _addedlayer))
              (Class|ConstraintInstanceBlueprintLibrary|GetLinearLimits _returnvalue_13)
              (Utilities|Array|Add (Variables|Default|GetAnchorArray) _outhit_impactpoint)))
          (:then_1
            (Variables|Default|SetLastSpeed (Transformation|GetComponentVelocity (Variables|Default|GetFuckEpics)))
            (if (Variables|Default|GetUpdateLength)
              (bind _returnvalue_14 (Class|PhysicsConstraintComponent|GetConstraint _addedlayer))
              (bind _limit_3 (Class|ConstraintInstanceBlueprintLibrary|GetLinearLimits _returnvalue_14))
              (Class|PhysicsConstraintComponent|SetLinearXLimit _addedlayer "LCM_Limited" (Math|Float|SelectFloat _returnvalue_8 _limit_3 (< _returnvalue_8 _limit_3))))))
        (else
          (Actor|DestroyActor))))))

(event EventBeginPlay
  (bind _addedlayer (Variables|Default|GetAddedLayer))
  (bind _asbase_drone (Utilities|Casting|CastToBaseDrone (Variables|Actor|GetInstigator)))
  (bind _output_get (Variables|Default|SetGrappler _asbase_drone))
  (Transformation|SetRelativeLocation (Variables|Default|GetFuckEpics) (Transformation|GetActorLocation _output_get) false true)
  (Class|PhysicsConstraintComponent|SetConstraintReferencePosition _addedlayer "Frame1" (Math|Vector|MakeVector 0.0 0.0 0.0))
  (Class|PhysicsConstraintComponent|SetLinearXLimit _addedlayer "LCM_Limited" (Variables|Default|GetConstructGrappleLength))
  (Transformation|AttachComponentToComponent (Variables|Default|GetGrappler) (Variables|Default|GetFuckEpics) "None" "KeepWorld" "KeepWorld" "KeepWorld" true)
  (Physics|AddForce (Variables|Default|GetFuckEpics) (* (Variables|Default|GetForce) 100) "None" true)
  (Development|PrintString (Utilities|GetDisplayName (Game|GetInstigator))))

(fn ConstructionScript)

(fn Trace
  (params (Start :type Vector) (End :type Vector) (ActorsToIgnore :type Array%20of%20Actor%20Object%20References))
  (bind _debugtrace (LocalVariables|GetDEBUGTRACE))
  (bind _precisionrad (Variables|Default|GetPrecisionRad))
  (bind (_outhit _returnvalue) (Collision|SphereTraceByChannel Start End _precisionrad "TraceTypeQuery1" false ActorsToIgnore _debugtrace true "(R=0.965394,G=0.000000,B=1.000000,A=1.000000)" "(R=1.000000,G=0.904667,B=0.000000,A=1.000000)"))
  (bind (_outhit_2 _returnvalue_2) (Collision|SphereTraceByChannel End Start _precisionrad "TraceTypeQuery1" false ActorsToIgnore _debugtrace))
  (return (+ (/ (+ (.location _outhit) (.location _outhit_2)) 2) (* (/ (+ (.normal _outhit) (.normal _outhit_2)) (Math|Vector|VectorLength (+ (.normal _outhit) (.normal _outhit_2)))) (Variables|Default|GetPrecisionRad))) (and _returnvalue _returnvalue_2)))