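; BP_BaseEnvironmentObject is a base Blueprint for physics-driven environment objects that expose damage reduction values.
; Its construction script makes the mesh simulate physics with query-and-physics collision and overlap events, blocking every channel except GameTraceChannel1, which it overlaps.
; Two getters return the flat and percentage damage reduction variables; no damage is applied here.
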(fn ConstructionScript
  (bind _mesh (Variables|Default|GetMesh))
  (Physics|SetSimulatePhysics _mesh true)
  (Collision|SetCollisionEnabled _mesh "QueryAndPhysics")
  (Variables|/Script/Engine.PrimitiveComponent|SetbGenerateOverlapEvents _mesh true)
  (Collision|SetCollisionResponsetoAllChannels _mesh "ECR_Block")
  (Collision|SetCollisionResponsetoChannel _mesh "ECC_GameTraceChannel1" "ECR_Overlap"))

(fn GetFlatDamageReduction
  (return (Variables|Default|GetFlatDamageReduction)))

(fn GetPercentageDamageReduction
  (return (Variables|Default|GetPercentageDamageReduction)))