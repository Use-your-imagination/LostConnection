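; BP_DevPlayerController is a debug player controller built to load and spawn the SN4K3 drone.
; Its loading events load primary assets and the SN4K3 data asset, then initialize the LostConnection player state and spawn the drone at a PlayerStart for this controller.
; The loading-screen setup that binds these events as callbacks is disconnected, and BeginPlay is empty, so nothing here triggers the sequence.
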(event Custom|BeginAssetsLoading
  (Utilities|LoadPrimaryAssets
    (:out
      (Utilities|LoadDroneAsset "/Script/LostConnection.SN4K3DataAsset"))))

(event Custom|EndAssetsLoading
  (bind _asbp_lost_connection_player_state (Utilities|Casting|CastToBP_LostConnectionPlayerState (Variables|GetPlayerState)))
  (Class|LostConnectionPlayerState|Init _asbp_lost_connection_player_state)
  (CallFunction|Spawn self))

(event Custom|Spawn
  (params (Contoller :type Player%20Controller%20Object%20Reference))
  (bind _returnvalue (Actor|GetActorOfClass "/Script/Engine.PlayerStart"))
  (Class|UtilityBlueprintFunctionLibrary|SpawnDrone "/Game/Drones/SN4K3/BP_SN4K3.BP_SN4K3_C" (Transformation|GetActorTransform _returnvalue) Contoller))

(event EventBeginPlay)

(fn ConstructionScript)