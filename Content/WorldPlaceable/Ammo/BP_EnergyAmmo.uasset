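; BP_EnergyAmmo is a world-placeable energy ammo actor that visually reflects how much ammo remains.
; On BeginPlay it plays a drop montage on its skeletal mesh.
; When the ammo mesh state changes, it plays an update montage and destroys the First component at Mid, or both Second and any remaining First component at Empty.
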(event EventBeginPlay
  (Animation|Montage|PlayMontage (Variables|Character|GetMesh) "/Game/Assets/Weapons/Ammo/EnergyAmmo/Animations/EnergyAmmo_Drop_Montage.EnergyAmmo_Drop_Montage"))

(event EventOnAmmoMeshChange
  (params (currentMesh :type Skeletal%20Mesh%20Object%20Reference))
  (bind _first (Variables|Default|GetFirst))
  (Animation|Montage|PlayMontage (Variables|Character|GetMesh) "/Game/Assets/Weapons/Ammo/EnergyAmmo/Animations/EnergyAmmo_Update_Montage.EnergyAmmo_Update_Montage"
    (:then
      (if (== currentMesh (Variables|Default|Getmid))
        (Components|DestroyComponent _first)
        (elif (== currentMesh (Variables|Default|Getempty))
          (Components|DestroyComponent (Variables|Default|GetSecond))
          (if (Utilities|IsValid _first)
            (Components|DestroyComponent (Variables|Default|GetFirst))))))))

(fn ConstructionScript)