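; BP_LostConnectionGameMode is a game mode that sets up the player's HUD when play begins.
; It casts the player pawn to BP_BaseDrone, then creates, displays and stores a BP_LostConnectionUI widget.
; It also switches language and locale to English without saving to config.
; A dynamic instance of the weapon circular selector material becomes the selector's brush and is stored as SelectorMaterial.
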(event EventBeginPlay
  (bind _asbp_base_drone (Utilities|Casting|CastToBP_BaseDrone (Game|Player|GetPlayerPawn 0)))
  (bind _returnvalue (UserInterface|CreateWidget "/Game/UI/BP_LostConnectionUI.BP_LostConnectionUI_C" 0 _asbp_base_drone))
  (UserInterface|Viewport|AddtoViewport _returnvalue 0)
  (Variables|Default|SetCurrentUI _returnvalue)
  (Class|KismetInternationalizationLibrary|SetCurrentLanguageandLocale (Utilities|String|MakeLiteralString "EN_us"))
  (bind _returnvalue_2 (Rendering|Material|CreateDynamicMaterialInstance "/Game/UI/WeaponCircularSelector/MWeaponCircularSelector.MWeaponCircularSelector" "None" "None" :!class /Script/Engine.KismetMaterialLibrary))
  (Class|Image|SetBrush (Variables|/Game/UI/WeaponCircularSelector/BP_WeaponCircularSelector.BP_WeaponCircularSelector_C|GetSelector (Variables|/Game/UI/BP_LostConnectionUI.BP_LostConnectionUI_C|GetWeaponCircularSelector (Variables|Default|GetCurrentUI))) (Class|WidgetBlueprintLibrary|MakeBrushfromMaterial _returnvalue_2 250 250))
  (Variables|Default|SetSelectorMaterial _returnvalue_2))

(fn ConstructionScript)