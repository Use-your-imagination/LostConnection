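; Player character Blueprint for a third-person shooter with firing, reload, ADS zoom, slide, ground slam, wallrun, ragdoll death and a pause-menu toggle.
; Input and hit events call dispatchers bound at BeginPlay to per-ability graphs, while AnimBP callbacks move the magazine and end slides.
; Timers drive fire montages, camera arm/FOV blends, slide checks and wall traces.
; Wallrun only tracks wall contact and rotation state; its break handler is empty.
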(event Custom|LHMag
  ;[1 1 1] Begin Play Event
  ;;[1 1 1] Inherent Binders
  (Transformation|AttachComponentToComponent (Variables|Default|Getmagazine) (Variables|Character|GetMesh) "hand_l" "KeepRelative" "KeepRelative" "KeepRelative" true))

(event Custom|WeaponMag
  ;[1 1 1] Begin Play Event
  ;;[1 1 1] Inherent Binders
  (Transformation|AttachComponentToComponent (Variables|Default|Getmagazine) (Variables|Default|GetcurrentWeaponMesh) "magazine" "KeepRelative" "KeepRelative" "KeepRelative" true))

(event Custom|BreakSlide
  ;[1 1 1] Begin Play Event
  ;;[1 1 1] Inherent Binders
  (Default|CallSlideBreak))

(event Custom|ShootAnim
  ;[0 1 0] Fire anim R2G
  (if (Class|LostConnectionCharacter|IsWeaponEquipped)
    (if (Variables|Inputs|GetPrimaryHold)
      (Animation|PlayAnimMontage "/Game/Mannequin/Animations/Fire_Rifle_Hip_Montage.Fire_Rifle_Hip_Montage" (/ (Math|Conversions|ToFloat(Integer) (Class|BaseWeapon|GetRateOfFire (Variables|Default|GetcurrentWeapon))) (/ 1.0 0.23)) "None"))))

(event EventTick
  (params (DeltaSeconds :type Float%20%28single-precision%29))
  (bind _capsulecomponent (Variables|Default|GetCapsuleComponent))
  (Utilities|FlowControl|Sequence
    (:then_0
      (if (and (Class|LostConnectionCharacter|IsWeaponEquipped) (Variables|Zoom|GetZooming))
        (bind _outhit_location (CallFunction|Lookingat (Variables|Default|GetFollowCamera) "None" 1e+04))
        (Transformation|SetWorldRotation _capsulecomponent (Math|Rotator|MakeRotator 0.0 0.0 (.yaw (Math|Conversions|RotationFromXVector (- _outhit_location (Transformation|GetWorldLocation _capsulecomponent))))) false false)
        (goto _label Reset)
        (else
          (Utilities|FlowControl|DoOnce false :!label _label
            (:Completed
              (Default|CallZoomBreak))))))))

(event EventBeginPlay
  ;[1 1 1] Begin Play Event
  (Utilities|FlowControl|Sequence
    (:then_0
      ;;[1 1 1] Setters
      (bind _asanimation_bp_lost_connection_character (Utilities|Casting|CastToAnimationBP_LostConnectionCharacter (Components|SkeletalMesh|GetAnimInstance (Variables|Character|GetMesh))))
      (Variables|Default|SetAnimBP _asanimation_bp_lost_connection_character))
    (:then_1
      ;;[1 1 1] Inherent Binders
      (EventDispatchers|AssignLHMag (Variables|Default|GetAnimBP) (delegate Custom|LHMag))
      (EventDispatchers|AssignWeaponMag (Variables|Default|GetAnimBP) (delegate Custom|WeaponMag))
      (EventDispatchers|AssignSlideBreak (Variables|Default|GetAnimBP) (delegate Custom|BreakSlide)))
    (:then_2
      ;;[1 1 1] Owning Binders
      (Utilities|FlowControl|Sequence
        (:then_0
          ;;;[1 1 1] Slide
          (EventDispatchers|BindEventtoSlideBreak (delegate SlideBreaker))
          (EventDispatchers|BindEventtoSlideInit (delegate SlideIniter))
          (EventDispatchers|BindEventtoGroundSlamInit (delegate GroundSlamIninter))
          ;;;[1 1 1] Zoom
          (EventDispatchers|BindEventtoZoomInit (delegate ZoomIniter))
          (EventDispatchers|BindEventtoZoomBreak (delegate ZoomBreaker)))
        (:then_1
          (Collision|AssignOnActorHit (delegate WallrunHiter))
          (EventDispatchers|AssignWallrunInit (delegate WallrunIniter))
          (EventDispatchers|BindEventtoWallrunBreak (delegate WallrunBreaker)))))))

(event Input|ActionEvents|InputActionMenu
  (params (Key :type Key%20Structure :default "None"))
  ;[0 1 0] ESC Menu
  (:Pressed
    (bind _asplayer_controller (Utilities|Casting|CastToPlayerController (Pawn|GetController)))
    (bind _asbp_hud (Utilities|Casting|CastToBP_HUD (HUD|GetHUD _asplayer_controller)))
    (switch Utilities|FlowControl|Switch|SwitchonESlateVisibility (Widget|GetVisibility (Variables|/Game/HUD/UI/BP_LostConnectionUI.BP_LostConnectionUI_C|GetMenu (Variables|/Game/HUD/BP_HUD.BP_HUD_C|GetCurrentUI _asbp_hud)))
      (:Visible
        (Widget|SetVisibility (Variables|/Game/HUD/UI/BP_LostConnectionUI.BP_LostConnectionUI_C|GetMenu (Variables|/Game/HUD/BP_HUD.BP_HUD_C|GetCurrentUI _asbp_hud)) "Hidden")
        (Variables|/Script/Engine.PlayerController|SetbShowMouseCursor _asplayer_controller false)
        (Input|SetInputModeGameOnly _asplayer_controller)
        (Default|DeletePopupWindow (Variables|/Game/HUD/BP_HUD.BP_HUD_C|GetCurrentUI _asbp_hud))
        (Game|SetGamePaused false))
      (:Hidden
        (Widget|SetVisibility (Variables|/Game/HUD/UI/BP_LostConnectionUI.BP_LostConnectionUI_C|GetMenu (Variables|/Game/HUD/BP_HUD.BP_HUD_C|GetCurrentUI _asbp_hud)) "Visible")
        (Variables|/Script/Engine.PlayerController|SetbShowMouseCursor _asplayer_controller true)
        (Input|SetInputModeGameandUI _asplayer_controller 0 "DoNotLock" false)
        (Game|SetGamePaused true)))))

(event Input|ActionEvents|InputActionZoom
  (params (Key :type Key%20Structure :default "None"))
  ;[1 1 1] ADS WIP
  (:Pressed
    (Variables|Inputs|SetSecondaryHold true)
    (Default|CallZoomInit))
  (:Released
    (Variables|Inputs|SetSecondaryHold false)
    (Default|CallZoomBreak)))

(event Input|ActionEvents|InputActionCrouch
  (params (Key :type Key%20Structure :default "None"))
  (bind _slidecooldownduration (Variables|CrouchandSlide|GetSlideCooldownDuration))
  ;[1 1 1] Crouch & Ground Slam WIP
  ;;[1 1 1] CrouchInput
  (:Pressed
    (Variables|Inputs|SetCrouchHold true)
    (if (AI|Components|NavMovement|IsFalling (Variables|Character|GetCharacterMovement))
      (if (< (.pitch (Transformation|GetWorldRotation (Variables|Default|GetFollowCamera))) -75.0)
        (Default|CallGroundSlamInit)
        (else
          (Default|CallSlideInit _slidecooldownduration)))
      (else
        (Character|Crouch)
        (if (Variables|Inputs|GetSprintHold)
          (Default|CallSlideInit _slidecooldownduration)))))
  (:Released
    (Variables|Inputs|SetCrouchHold false)
    (if (== (Utilities|Time|GetTimerRemainingTimebyHandle (Variables|CrouchAndSlide|GetSlideActivityHandle)) 0.0)
      (Character|UnCrouch))))

(event Input|KeyboardEvents|R
  (params (Key :type Key%20Structure :default "None"))
  ;[0 1 0] Reload R2G
  (:Pressed
    (if (not (Variables|Default|GetIsReloading))
      (Animation|PlayAnimMontage "/Game/Mannequin/Animations/Reload_Rifle_Hip_Montage.Reload_Rifle_Hip_Montage" 3.0 "")
      (Variables|Default|SetIsReloading true))))

(event Input|KeyboardEvents|X
  (params (Key :type Key%20Structure :default "None"))
  (bind _currentweaponmesh (Variables|Default|GetcurrentWeaponMesh))
  (bind _mesh (Variables|Character|GetMesh))
  ;[0 1 0] Death ragdoll R2G
  (:Pressed
    (Utilities|FlowControl|Sequence
      (:then_0
        (Transformation|DetachFromComponent _currentweaponmesh "KeepWorld" "KeepWorld" "KeepWorld" true)
        (Collision|SetCollisionEnabled _currentweaponmesh "PhysicsOnly")
        (Physics|SetSimulatePhysics _currentweaponmesh true)
        (Collision|SetCollisionEnabled (Variables|Default|Getmagazine) "NoCollision")
        (Collision|SetCollisionEnabled _mesh "PhysicsOnly")
        (Physics|SetSimulatePhysics _mesh true)
        (Pawn|Components|CharacterMovement|DisableMovement (Variables|Character|GetCharacterMovement)))
      (:then_1
        ;;[1 0.1039 0.9173] Just fancy shit
        (Niagara|SpawnSystemAttached "/Game/Assets/FX/NPS_Death.NPS_Death" (Variables|Character|GetMesh) "None" "0, 0, 0" "0, 0, 0" "KeepRelativeOffset" false)))))

(event Input|MouseEvents|LeftMouseButton
  (params (Key :type Key%20Structure :default "None"))
  ;[0 1 0] Fire anim R2G
  (:Pressed
    (if (Class|LostConnectionCharacter|IsWeaponEquipped)
      (Variables|Inputs|SetPrimaryHold true)
      (bind _returnvalue (Utilities|Time|SetTimerbyEvent (delegate Custom|ShootAnim) (/ 1.0 (Math|Conversions|ToFloat(Integer) (Class|BaseWeapon|GetRateOfFire (Variables|Default|GetcurrentWeapon)))) true))
      (else
        (Variables|Inputs|SetPrimaryHold false :!label _label)
        (Utilities|Time|ClearandInvalidateTimerbyHandle _returnvalue))))
  (:Released
    (goto _label)))

(event Input|KeyboardEvents|LeftShift
  (params (Key :type Key%20Structure :default "None"))
  ;[1 1 1] Shift
  (:Pressed
    (Variables|Inputs|SetSprintHold true))
  (:Released
    (Variables|Inputs|SetSprintHold false)))

(fn ConstructionScript)

(fn Lookingat
  (params (WhoIsLooking :type Camera%20Component%20Object%20Reference) (DrawType :type EDrawDebugTrace%20Enum :default "None") (Distance :type Float%20%28single-precision%29))
  (bind _returnvalue (Transformation|GetWorldRotation WhoIsLooking))
  (bind _returnvalue_2 (Transformation|GetWorldLocation WhoIsLooking))
  (bind _returnvalue_3 (Math|Vector|GetForwardVector _returnvalue))
  (bind _returnvalue_4 (* _returnvalue_3 Distance))
  (bind (_outhit _returnvalue_5) (Collision|LineTraceByChannel _returnvalue_2 (+ _returnvalue_2 _returnvalue_4) "TraceTypeQuery1" false 0 DrawType true "(R=1.000000,G=0.000000,B=0.000000,A=1.000000)" "(R=0.000000,G=1.000000,B=0.000000,A=1.000000)" 1.0))
  (if _returnvalue_5
    (return (.location _outhit))
    (else
      (return _returnvalue_4))))

(event Custom|WallrunCheck
  (bind _returnvalue (Transformation|GetActorLocation))
  (bind _returnvalue_2 (Collision|LineTraceByChannel _returnvalue (+ _returnvalue (* (stale Custom|WallrunInit_Event _output_get) (* (+ (Components|Capsule|GetScaledCapsuleRadius (Variables|Default|GetCapsuleComponent)) 5.0) -1.0))) "TraceTypeQuery1" false 0 "None"))
  (if (not _returnvalue_2)
    (Default|CallWallrunBreak)))

(event Custom|WallrunInit_Event
  (params (HitResult :type Hit%20Result%20Structure))
  (bind _impactnormal (Collision|BreakHitResult HitResult))
  (bind _returnvalue (Math|Conversions|RotationFromXVector _impactnormal))
  (if (Math|Boolean|ANDBoolean (not (Variables|Wallrun|GetWallrun)) (Math|Float|NearlyEqual(Float) (.roll _returnvalue) 0.0 1e-06) (Math|Float|NearlyEqual(Float) (.pitch _returnvalue) 0.0 1e-06))
    (Default|CallZoomBreak)
    (bind _output_get (Variables|Default|SetCurrentWallNormal _impactnormal))
    (Variables|/Script/Engine.CharacterMovementComponent|SetbOrientRotationToMovement (Variables|Character|GetCharacterMovement) false)
    (Variables|Wallrun|SetWallrun true)
    (Utilities|Time|SetTimerbyEvent (delegate Custom|WallrunCheck) 0.02 true)))

(event Custom|WallrunHit_Event
  (params (SelfActor :type Actor%20Object%20Reference) (OtherActor :type Actor%20Object%20Reference) (NormalImpulse :type Vector) (Hit :type Hit%20Result%20Structure%20%28by%20ref%29))
  (Default|CallWallrunInit Hit))

(event Custom|SlideBreak_Event
  (bind _charactermovement (Variables|Character|GetCharacterMovement))
  (Variables|/Script/Engine.CharacterMovementComponent|SetBrakingFrictionFactor _charactermovement 2.0)
  (Variables|/Script/Engine.CharacterMovementComponent|SetBrakingDecelerationWalking _charactermovement 2048.0)
  (Variables|/Script/Engine.CharacterMovementComponent|SetRotationRate _charactermovement (Math|Rotator|MakeRotator 0.0 0.0 5.4e+02)))

(event Custom|WallrunBreak_Event)

(event Custom|ZoomBreak_Event
  (Variables|/Script/Engine.CharacterMovementComponent|SetbOrientRotationToMovement (Variables|Character|GetCharacterMovement) true)
  (|ZoomOUT (Variables|Zoom|GetCameraArmZoom) (Variables|Zoom|GetCameraArmDefault) (Variables|Zoom|GetCameraFOVZoom) (Variables|Zoom|GetCameraFOVDefault)
    (:NewParam
      (Variables|Zoom|SetZooming false))))

(event Custom|ZoomOUTBreak_Event
  (Utilities|Time|ClearandInvalidateTimerbyHandle (stale _returnvalue)))

(event Custom|ZoomOUTER
  (bind _followcamera (Variables|Default|GetFollowCamera))
  (bind _cameraoffset (Variables|Default|GetCameraOffset))
  (bind _fieldofview (Variables|/Script/Engine.CameraComponent|GetFieldOfView _followcamera))
  (if (or (> (stale _toarm) (Variables|/Script/Engine.SpringArmComponent|GetTargetArmLength _cameraoffset)) (> (stale _tofov) _fieldofview))
    (Variables|/Script/Engine.SpringArmComponent|SetTargetArmLength _cameraoffset (- (Variables|/Script/Engine.SpringArmComponent|GetTargetArmLength _cameraoffset) (/ (- (stale _fromarm) (stale _toarm)) (/ (Variables|Zoom|GetZoomTime) (+ (Class|KismetSystemLibrary|GetTimerElapsedTimeHandle (stale _returnvalue)) (Utilities|Time|GetTimerRemainingTimebyHandle (stale _returnvalue)))))))
    (Camera|SetFieldOfView _followcamera (- _fieldofview (/ (- (stale _fromfov) (stale _tofov)) (/ (Variables|Zoom|GetZoomTime) (+ (Class|KismetSystemLibrary|GetTimerElapsedTimeHandle (stale _returnvalue)) (Utilities|Time|GetTimerRemainingTimebyHandle (stale _returnvalue)))))))
    (else
      (Variables|/Script/Engine.SpringArmComponent|SetTargetArmLength _cameraoffset (stale _toarm))
      (Camera|SetFieldOfView _followcamera (stale _tofov))
      (Utilities|Time|ClearandInvalidateTimerbyHandle (stale _returnvalue)))))

(event Custom|ZoomInit_Event
  (if (and (Class|LostConnectionCharacter|IsWeaponEquipped) (not false))
    (Variables|/Script/Engine.CharacterMovementComponent|SetbOrientRotationToMovement (Variables|Character|GetCharacterMovement) false)
    (|ZoomIN (Variables|Zoom|GetCameraArmDefault) (Variables|Zoom|GetCameraArmZoom) (Variables|Zoom|GetCameraFOVDefault) (Variables|Zoom|GetCameraFOVZoom)
      (:NewParam
        (Variables|Zoom|SetZooming true)))))

(event Custom|ZoomINBreak_Event
  (Utilities|Time|ClearandInvalidateTimerbyHandle (stale _returnvalue)))

(event Custom|ZoomINER
  (bind _followcamera (Variables|Default|GetFollowCamera))
  (bind _cameraoffset (Variables|Default|GetCameraOffset))
  (bind _fieldofview (Variables|/Script/Engine.CameraComponent|GetFieldOfView _followcamera))
  (if (Variables|Inputs|GetSecondaryHold)
    (if (or (> (Variables|/Script/Engine.SpringArmComponent|GetTargetArmLength _cameraoffset) (stale _toarm)) (> _fieldofview (stale _tofov)))
      (Variables|/Script/Engine.SpringArmComponent|SetTargetArmLength _cameraoffset (- (Variables|/Script/Engine.SpringArmComponent|GetTargetArmLength _cameraoffset) (/ (- (stale _fromarm) (stale _toarm)) (/ (Variables|Zoom|GetZoomTime) (+ (Class|KismetSystemLibrary|GetTimerElapsedTimeHandle (stale _returnvalue)) (Utilities|Time|GetTimerRemainingTimebyHandle (stale _returnvalue)))))))
      (Camera|SetFieldOfView _followcamera (- _fieldofview (/ (- (stale _fromfov) (stale _tofov)) (/ (Variables|Zoom|GetZoomTime) (+ (Class|KismetSystemLibrary|GetTimerElapsedTimeHandle (stale _returnvalue)) (Utilities|Time|GetTimerRemainingTimebyHandle (stale _returnvalue)))))))
      (else
        (Variables|/Script/Engine.SpringArmComponent|SetTargetArmLength _cameraoffset (stale _toarm))
        (Camera|SetFieldOfView _followcamera (stale _tofov))
        (Utilities|Time|ClearandInvalidateTimerbyHandle (stale _returnvalue))))))

(event Custom|GroundSlamInit_Event
  (bind _returnvalue (Transformation|GetActorLocation))
  (bind (_outhit _returnvalue_2) (Collision|CapsuleTraceByChannel _returnvalue (+ _returnvalue (* (Math|Vector|VectorDown) (Variables|CrouchAndSlide|GetGroundSlamMaxHight))) (Components|Capsule|GetScaledCapsuleRadius (Variables|Default|GetCapsuleComponent)) 0.0 "TraceTypeQuery1" false 0 "None"))
  (if _returnvalue_2
    (Variables|/Script/Engine.MovementComponent|SetVelocity (Variables|Character|GetCharacterMovement) (* (- (.location _outhit) _returnvalue) (/ (.distance _outhit) (Variables|CrouchandSlide|GetGroundSlamContolValue))))))

(event Custom|SlideCooldownEnd
  (Variables|CrouchAndSlide|SetSlideCooldown false))

(event Custom|SlideInit_Event
  (params (SlideCooldownDuration :type Float%20%28single-precision%29))
  (bind _returnvalue (Transformation|GetVelocity))
  (bind _charactermovement (Variables|Character|GetCharacterMovement))
  (bind _charactermovement_2 (Variables|Character|GetCharacterMovement))
  (if (not (Variables|CrouchAndSlide|GetSlideCooldown))
    (if (not (AI|Components|NavMovement|IsFalling _charactermovement_2))
      (Variables|/Script/Engine.CharacterMovementComponent|SetBrakingFrictionFactor _charactermovement_2 0.15)
      (Variables|/Script/Engine.CharacterMovementComponent|SetBrakingDecelerationWalking _charactermovement_2 0.0)
      (Variables|/Script/Engine.MovementComponent|SetVelocity _charactermovement (/ _returnvalue (/ (Math|Vector|VectorLength _returnvalue) (/ (Variables|CrouchandSlide|GetSlideSpeed) (Variables|CrouchAndSlide|GetSlideAirSpeedScale)))))
      (Variables|/Script/Engine.CharacterMovementComponent|SetRotationRate _charactermovement_2 (Math|Rotator|MakeRotator 0.0 0.0 (Variables|CrouchAndSlide|GetSlideRotationRate)))
      (else
        (bind _outhit_location (CallFunction|Lookingat (Variables|Default|GetFollowCamera) "None" 1e+04))
        (Variables|/Script/Engine.MovementComponent|SetVelocity _charactermovement (/ (- _outhit_location (Transformation|GetWorldLocation (Variables|Default|GetCapsuleComponent))) (/ (Math|Vector|VectorLength (- _outhit_location (Transformation|GetWorldLocation (Variables|Default|GetCapsuleComponent)))) (Variables|CrouchandSlide|GetSlideSpeed))))))
    (Variables|CrouchAndSlide|SetSlideCooldown true)
    (bind _returnvalue_2 (Utilities|Time|SetTimerbyEvent (delegate Custom|SlideCooldownEnd) SlideCooldownDuration))
    (Variables|CrouchAndSlide|SetSlideCooldownHandle _returnvalue_2)
    (bind _returnvalue_3 (Utilities|Time|SetTimerbyEvent (delegate Custom|SlideBreakByMS) 0.25 true))
    (Variables|CrouchAndSlide|SetSlideActivityHandle _returnvalue_3)))

(event Custom|SlideBreakByMS
  (bind _returnvalue (Transformation|GetVelocity))
  (if (< (Math|Vector|VectorLength (Math|Vector|MakeVector (.x _returnvalue) (.y _returnvalue) 0.0)) 375.0)
    (Utilities|Time|ClearandInvalidateTimerbyHandle (Variables|CrouchAndSlide|GetSlideActivityHandle))
    (Default|CallSlideBreak)
    (if (not (Variables|Inputs|GetCrouchHold))
      (Character|UnCrouch))))