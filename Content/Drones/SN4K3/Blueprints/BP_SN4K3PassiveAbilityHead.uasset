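; Player-steered flying head for the SN4K3 drone's passive ability, which flies forward once activated and explodes on impact.
; Speedup boosts fly speed and acceleration, cutting turn and look input to a twentieth.
; On the authority, capsule overlaps with non-ally targetable actors or environment objects trigger the explosion.
; Explode and speedup checks extend the parent's, also requiring a hidden escape menu.
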(event OnComponentBeginOverlap(CapsuleComponent)
  (params (OverlappedComponent :type Primitive%20Component%20Object%20Reference) (OtherActor :type Actor%20Object%20Reference) (OtherComp :type Primitive%20Component%20Object%20Reference) (OtherBodyIndex :type Integer) (bFromSweep :type Boolean) (SweepResult :type Hit%20Result%20Structure%20%28by%20ref%29))
  (Networking|SwitchHasAuthority
    (:Authority
      ;[1 1 1] BUG can proc before spawn
      (bind _asaitargeted (Utilities|Casting|CastToAITargeted OtherActor)
        (:then
          (if (not (Class|AITargeted|GetIsAlly _asaitargeted))
            (Class|SN4K3PassiveAbilityHead|Explode :!label _label)))
        (:CastFailed
          (Utilities|Casting|CastToBP_BaseEnvironmentObject OtherActor)
          (goto _label))))))

(event Custom|Activate
  (Variables|Default|SetActivated true))

(event EventSpeedup
  (bind _charactermovement (Variables|Character|GetCharacterMovement))
  (if (Variables|Default|GetActivated)
    (Variables|/Script/Engine.CharacterMovementComponent|SetMaxFlySpeed _charactermovement 3.2e+03)
    (Variables|/Script/Engine.CharacterMovementComponent|SetMaxAcceleration _charactermovement 1.2e+04)
    (Variables|Default|SetAccelerated true)))

(event EventTick
  (params (DeltaSeconds :type Float%20%28single-precision%29))
  (if (Variables|Default|GetActivated)
    (Pawn|Input|AddMovementInput (Transformation|GetActorForwardVector) 1.0 false)))

(event Input|AxisEvents|InputAxisTurn
  (params (AxisValue :type Float%20%28single-precision%29))
  (Pawn|Input|AddControllerYawInput (Math|Float|SelectFloat (/ AxisValue 2e+01) AxisValue (Variables|Default|GetAccelerated))))

(event Input|AxisEvents|InputAxisLookUp
  (params (AxisValue :type Float%20%28single-precision%29))
  (Pawn|Input|AddControllerPitchInput (Math|Float|SelectFloat (/ AxisValue 2e+01) AxisValue (Variables|Default|GetAccelerated))))

(fn ConstructionScript)

(fn CheckExplode
  (bind _returnvalue (|CallParentFunction))
  (bind _asbp_lost_connection_player_state (Utilities|Casting|CastToBP_LostConnectionPlayerState (Variables|Default|GetPlayerState)))
  (bind _asiescape_menu_holder (Utilities|Casting|CastToIEscapeMenuHolder (Variables|/Script/LostConnection.LostConnectionPlayerState|GetcurrentUI _asbp_lost_connection_player_state)))
  (bind _escapemenu (Default|GetEscapeMenu _asiescape_menu_holder))
  (return (and _returnvalue (Utilities|Enum|Equal(Enum) (Widget|GetVisibility _escapemenu) "Hidden"))))

(fn CheckSpeedup
  (bind _returnvalue (|CallParentFunction))
  (bind _asbp_lost_connection_player_state (Utilities|Casting|CastToBP_LostConnectionPlayerState (Variables|Default|GetPlayerState)))
  (bind _asiescape_menu_holder (Utilities|Casting|CastToIEscapeMenuHolder (Variables|/Script/LostConnection.LostConnectionPlayerState|GetcurrentUI _asbp_lost_connection_player_state)))
  (bind _escapemenu (Default|GetEscapeMenu _asiescape_menu_holder))
  (return (and _returnvalue (Utilities|Enum|Equal(Enum) (Widget|GetVisibility _escapemenu) "Hidden"))))