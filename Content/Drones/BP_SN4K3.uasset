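; Player Blueprint for the SN4K3 drone, a shooter character with zoom, crouch, slide, jump, wallrun, weapon selection and a menu toggle.
; The event graph is a thin dispatcher, passing input, tick, timer, reload and death events to external functions with itself as argument.
; A bound hit event on the wallrun hitter starts wallruns, and a cooldown event unblocks them.
; Two getters expose the passive ability's nanite meter as percent and text.
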(event EventPressWeaponSelectorAction
  (CallFunction|PressWeaponSelector self))

(event EventReleaseWeaponSelectorAction
  (CallFunction|ReleaseWeaponSelector self))

(event EventReloadEventVisual
  (CallFunction|ReloadVisual self))

(event EventReleaseShoot
  (CallFunction|ReleaseShoot self))

(event EventZoomTimerUpdate
  (CallFunction|ZoomUpdate self))

(event EventSlideTimerUpdate
  (CallFunction|SlideUpdate self))

(event EventTick
  (params (DeltaSeconds :type Float%20%28single-precision%29))
  (CallFunction|TickUpdate self))

(event EventBeginPlay
  (Collision|AssignOnActorHit (delegate WallrunHiter_2)))

(event EventWallrunTimerUpdate
  (CallFunction|WallrunUpdate self))

(event EventDeathMaterialTimerUpdate
  (CallFunction|DeathUpdate self))

(event EventShootTimerUpdate
  (CallFunction|ShootUpdate self))

(event EventWallrunCooldown
  (Variables|Default|SetwallrunBlocked false))

(event EventDeathEventVisual
  (CallFunction|DeathInit self))

(event EventPressZoomAction
  (CallFunction|Zoomin self))

(event EventPressJumpAction
  (CallFunction|PressJump self))

(event EventReleaseZoomAction
  (CallFunction|ZoomOut self))

(event EventPressCrouchAction
  (CallFunction|PressCrouch self))

(event EventReleaseCrouchAction
  (CallFunction|ReleaseCrouch self))

(event EventPressShoot
  (CallFunction|PressShoot self))

(event Input|ActionEvents|InputActionMenu
  (params (Key :type Key%20Structure :default "None"))
  (:Pressed
    (CallFunction|ChangeMenuVisibility self)))

(fn ConstructionScript)

(event Custom|WallrunHit_Event
  (params (SelfActor :type Actor%20Object%20Reference) (OtherActor :type Actor%20Object%20Reference) (NormalImpulse :type Vector) (Hit :type Hit%20Result%20Structure%20%28by%20ref%29))
  (CallFunction|WallrunInit self Hit))

(fn GetMeterPercent
  (bind _assn4k3passive_ability (Utilities|Casting|CastToSN4K3PassiveAbility (Variables|Default|GetpassiveAbility)))
  (return (/ (Math|Conversions|ToFloat(Integer) (Variables|/Script/LostConnection.SN4K3PassiveAbility|GetnaniteMeter _assn4k3passive_ability)) 1e+02)))

(fn GetMeterText
  (bind _assn4k3passive_ability (Utilities|Casting|CastToSN4K3PassiveAbility (Variables|Default|GetpassiveAbility)))
  (return (Utilities|Text|ToText(Integer) (Variables|/Script/LostConnection.SN4K3PassiveAbility|GetnaniteMeter _assn4k3passive_ability))))