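; Game instance for LostConnection that creates, finds and destroys LAN multiplayer sessions through Advanced Sessions nodes.
; CreateSession tags a four-slot session with a ServerName property, then on success opens the chosen level as a listen server and toggles the player character's menu visibility.
; FindSessions searches for a few LAN servers and writes the results into the SessionsData of the object passed in.
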(event Custom|CreateSession
  (params (LevelName :type Name%20%28by%20ref%29) (SessionName :type Name%20%28by%20ref%29))
  (bind _output_get (Variables|Default|SetLevelName LevelName))
  (|AdvancedSession (Utilities|Array|MakeArray (Class|AdvancedSessionsLibrary|MakeLiteralSessionPropertyString "ServerName" (Utilities|String|ToString(Name) SessionName))) (Game|GetPlayerController 0) 4 0 true false false true true false false false true
    (:OnSuccess
      (Game|OpenLevel(byName) _output_get true "?listen?bIsLanMatch=1")
      (bind _asbp_lost_connection_character (Utilities|Casting|CastToBP_LostConnectionCharacter (Game|Player|GetPlayerPawn 0)))
      (Default|ChangeMenuVisibility _asbp_lost_connection_character))))

(event Custom|FindSessions
  (params (Sessions :type BP%20Find%20Sessions%20Object%20Reference%20%28by%20ref%29))
  (bind _results (|FindSessionsAdvanced (Game|GetPlayerController 0) 5 true "AllServers" 0 false false false)
    (:OnSuccess
      (Variables|/Game/HUD/UI/PopupWindows/Multiplayer/BP_FindSessions.BP_FindSessions_C|SetSessionsData Sessions _results))))

(event Custom|DestroySession
  (|DestroySession (Game|GetPlayerController 0)))